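; Gameplay player controller for multiplayer that spawns the player character and handles the loading screen and in-game menu.
; On BeginPlay, a client event clears widgets, sets game-only input and calls the server, which reserves a free PlayerStart via its tag, spawns BP_Player there and possesses it.
; A separate client event shows the loading screen, while the menu input opens a UI-only menu with cursor and halts the character.
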(event `Server_SpawnCharacterOnServer`
  ;[1 1 1] Spawn character on server
  (`self.SpawnCharacter`))

(event `Client_CreateLoadingScreen`
  ;[1 1 1] Create loading screen on client
  (bind _returnvalue (`|CreateWidget` "/Game/Blueprints/Widgets/MultiplayerWidgets/WBP_LoadingScreen.WBP_LoadingScreen_C"))
  (`UserWidget.AddToViewport` _returnvalue 0))

(event `self.ReceiveBeginPlay`
  ;[1 1 1] BeginPlay, Spawn character
  (`self.Client_SpawnCharacterOnClient`))

(event `Client_SpawnCharacterOnClient`
  ;[1 1 1] Spawn character on client
  (`WidgetLayoutLibrary.RemoveAllWidgets`)
  (`self.Server_SpawnCharacterOnServer`)
  (`WidgetBlueprintLibrary.SetInputMode_GameOnly` self))

(event `EnhancedInput|/Game/Input/InputActions/IA_InGameMenu`
  (params (ActionValue :type Boolean) (ElapsedSeconds :type "Float (double-precision)") (TriggeredSeconds :type "Float (double-precision)") (InputAction :type "InputAction Object Reference" :default "/Game/Input/InputActions/IA_InGameMenu.IA_InGameMenu"))
  ;[1 1 1] Create In Game Menu
  (:`Triggered`
    (`self.CreateInGameMenu`)))

(fn `CreateInGameMenu`
  (bind _returnvalue (`GameplayStatics.GetPlayerCharacter` 0))
  ;[1 1 1] create in game menu, show mouse cursor and stop character movement
  (bind _returnvalue_2 (`|CreateWidget` "/Game/Blueprints/Widgets/MultiplayerWidgets/WBP_InGameMenu.WBP_InGameMenu_C"))
  (`UserWidget.AddToViewport` _returnvalue_2 0)
  (set `self.bShowMouseCursor` true)
  (`WidgetBlueprintLibrary.SetInputMode_UIOnlyEx` self _returnvalue_2)
  (`MovementComponent.StopMovementImmediately` (`Pawn.GetMovementComponent` _returnvalue))
  (`self.DisableInput` _returnvalue self))

(fn `SpawnCharacter`
  ;[1 1 1] Spawn actor and find free playerstart
  (bind _outactors (`GameplayStatics.GetAllActorsOfClass` "/Script/Engine.PlayerStart"))
  (for _array_element _outactors
    (if (!= (`PlayerStart.PlayerStartTag` _array_element) "Reserved")
      (set `PlayerStart.PlayerStartTag` "Reserved" _array_element)
      (break)))
  (bind _returnvalue (`|SpawnActorFromClass` "/Game/Blueprints/Characters/BP_Player.BP_Player_C" (`self.GetTransform` _array_element) "Undefined" "MultiplyWithRoot" null null))
  (`self.Possess` _returnvalue))

(fn `UserConstructionScript`)