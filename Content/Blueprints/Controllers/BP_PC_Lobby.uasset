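; Lobby player controller that manages each client's lobby UI, camera view and removal from the session.
; On BeginPlay it points the view at the first BP_C_Main actor.
; Client-prefixed events create the WBP_Lobby widget with UI-only input, then forward player list and map updates to it.
; Other events show a loading screen, or handle kicks by destroying the session and opening the main menu.
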(event `Client_KickPlayerFromTheLobby`
  ;[1 1 1] Kick player from the lobby
  (`DestroySessionCallbackProxy.DestroySession` self
    (:`then`
      (`GameplayStatics.OpenLevelBySoftObjectPtr` "/Game/Levels/Menus/MainMenu.MainMenu"))))

(event `self.ReceiveBeginPlay`
  ;[1 1 1] BeginPlay
  (`self.Client_SetNewViewTarget`))

(event `Client_AddNewPlayerToList`
  (params (LobbyPlayerName :type String) (LobbyPlayerIndex :type Integer))
  ;[1 1 1] Playerlist actions
  ;;[1 1 1] Add new players to the list
  (`/Game/Blueprints/Widgets/MultiplayerWidgets/WBP_Lobby.AddNewPlayersToList` (`self.WBP_Lobby`) LobbyPlayerName LobbyPlayerIndex))

(event `Client_CreateHUDAndSpawnCharacter`
  ;[1 1 1] Create lobby widget on client
  (bind _returnvalue (`|CreateWidget` "/Game/Blueprints/Widgets/MultiplayerWidgets/WBP_Lobby.WBP_Lobby_C"))
  (bind _output_get (set `self.WBP_Lobby` _returnvalue))
  (`UserWidget.AddToViewport` _output_get 0)
  (`WidgetBlueprintLibrary.SetInputMode_UIOnlyEx` (`GameplayStatics.GetPlayerController` 0) _output_get))

(event `Client_ClearAllPlayersFromTheList`
  ;[1 1 1] Playerlist actions
  ;;[1 1 1] Clear players from the list
  (`/Game/Blueprints/Widgets/MultiplayerWidgets/WBP_Lobby.ClearPlayersFromList` (`self.WBP_Lobby`)))

(event `Client_SetNewViewTarget`
  ;[1 1 1] Set new view target to main camera
  (bind _outactors (`GameplayStatics.GetAllActorsOfClass` "/Game/Blueprints/Cameras/BP_C_Main.BP_C_Main_C"))
  (`self.SetViewTargetWithBlend` (`|GetArrayItem` _outactors)))

(event `Client_CreateLoadingScreen`
  ;[1 1 1] Create loading screen on client
  (bind _returnvalue (`|CreateWidget` "/Game/Blueprints/Widgets/MultiplayerWidgets/WBP_LoadingScreen.WBP_LoadingScreen_C"))
  (`UserWidget.AddToViewport` _returnvalue 0))

(event `Client_UpdateMapInfoOnHUD`
  (params (S_Maps :type "/Game/Blueprints/Structures/S_Maps Structure"))
  ;[1 1 1] Update map information on client
  (`/Game/Blueprints/Widgets/MultiplayerWidgets/WBP_Lobby.UpdateMapInfo` (`self.WBP_Lobby`) S_Maps))

(fn `UserConstructionScript`)