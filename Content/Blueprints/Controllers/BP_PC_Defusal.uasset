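; Player controller for a bomb defusal mode, handling team selection, character spawning, HUD, loading screen and in-game menu.
; BeginPlay opens team selection; the client spawn event swaps widgets for the HUD and calls the server spawn.
; SpawnCharacter reserves a free team-tagged PlayerStart, spawns and possesses BP_Player, giving Terrorists the bomb; every character gets a red material.
; A ready check starts the round timer; the menu halts player movement and input.
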(event `self.ReceiveBeginPlay`
  ;[1 1 1] BeginPlay - AC
  (`self.Create Team Selection`))

(event `Check If Players Are Ready`
  (bind _returnvalue (`GameModeBase.GetNumPlayers` (`GameplayStatics.GetGameMode`)))
  (if (== (`self.Players_Ready`) _returnvalue)
    (`self.Start Round`)))

(event `Start Round`
  (set `self.Timer` 10))

(event `Server_SpawnCharacterOnServer`
  (params (Team :type "/Game/Blueprints/Characters/Enum_Team Enum" :default "NewEnumerator0"))
  ;[1 1 1] Spawn character on server
  (bind _bp_player (`self.SpawnCharacter` Team))
  (`self.Update Skin` _bp_player))

(event `Create Team Selection`
  ;[1 1 1] Create Team Selection Screen - AC
  (bind _returnvalue (`|CreateWidget` "/Game/Blueprints/Widgets/InGameWidgets/WBP_SelectTeam.WBP_SelectTeam_C"))
  (`UserWidget.AddToViewport` _returnvalue 0))

(event `Client_CreateLoadingScreen`
  ;[1 1 1] Create loading screen on client
  (bind _returnvalue (`|CreateWidget` "/Game/Blueprints/Widgets/MultiplayerWidgets/WBP_LoadingScreen.WBP_LoadingScreen_C"))
  (`UserWidget.AddToViewport` _returnvalue 0))

(event `Update Skin`
  (params (`BP Player` :type "/Game/Blueprints/Characters/BP_Player Object Reference"))
  (`PrimitiveComponent.SetMaterial` (`Character.Mesh` `BP Player`) 0 "/Game/3D/ThirdPersonCharacter/Materials/MI_UE4Man_Body_Red.MI_UE4Man_Body_Red"))

(event `EnhancedInput|/Game/Blueprints/Input/InputActions/IA_InGameMenu`
  (params (ActionValue :type Boolean) (ElapsedSeconds :type "Float (double-precision)") (TriggeredSeconds :type "Float (double-precision)") (InputAction :type "InputAction Object Reference" :default "/Game/Blueprints/Input/InputActions/IA_InGameMenu.IA_InGameMenu"))
  ;[1 1 1] Create In Game Menu
  (:`Triggered`
    (`self.CreateInGameMenu`)))

(event `Client_SpawnCharacterOnClient`
  (params (Team :type "/Game/Blueprints/Characters/Enum_Team Enum" :default "NewEnumerator0"))
  ;[1 1 1] Spawn character on client
  (`WidgetLayoutLibrary.RemoveAllWidgets`)
  (`self.Server_SpawnCharacterOnServer` Team)
  (`WidgetBlueprintLibrary.SetInputMode_GameOnly` self)
  (bind _returnvalue (`|CreateWidget` "/Game/Blueprints/Widgets/InGameWidgets/_WBP_HUD._WBP_HUD_C"))
  (`UserWidget.AddToViewport` _returnvalue 0))

(fn `CreateInGameMenu`
  (bind _returnvalue (`GameplayStatics.GetPlayerCharacter` 0))
  ;[1 1 1] create in game menu, show mouse cursor and stop character movement
  (bind _returnvalue_2 (`|CreateWidget` "/Game/Blueprints/Widgets/MultiplayerWidgets/WBP_InGameMenu.WBP_InGameMenu_C"))
  (`UserWidget.AddToViewport` _returnvalue_2 0)
  (set `self.bShowMouseCursor` true)
  (`WidgetBlueprintLibrary.SetInputMode_UIOnlyEx` self _returnvalue_2)
  (`MovementComponent.StopMovementImmediately` (`Pawn.GetMovementComponent` _returnvalue))
  (`self.DisableInput` _returnvalue self))

(fn `SpawnCharacter`
  (params (Team :type "/Game/Blueprints/Characters/Enum_Team Enum" :default "NewEnumerator0"))
  (returns (`BP Player` :type "/Game/Blueprints/Characters/BP_Player Object Reference"))
  ;[1 1 1] Spawn actor and find free playerstart
  (bind _outactors (`GameplayStatics.GetAllActorsOfClassWithTag` "/Script/Engine.PlayerStart" (`KismetStringLibrary.Conv_StringToName` (`|GetEnumeratorNameAsString` Team))))
  (for _array_element _outactors
    (if (!= (`PlayerStart.PlayerStartTag` _array_element) "Reserved")
      (set `PlayerStart.PlayerStartTag` "Reserved" _array_element)
      (break)))
  (bind _returnvalue (`|SpawnActorFromClass` "/Game/Blueprints/Characters/BP_Player.BP_Player_C" (`self.GetTransform` _array_element) "Undefined" "MultiplyWithRoot" null null))
  (bind _output_get (set `/Game/Blueprints/Characters/BP_Player.Team` Team _returnvalue))
  (switch `/Game/Blueprints/Characters/Enum_Team` _output_get
    (:`NewEnumerator0`
      (`/Game/Blueprints/Characters/BP_Player.SpawnWeapon` _returnvalue "/Game/Blueprints/Weapons/BP_Bomb.BP_Bomb_C" (0.0 0.0 0.0)))
    (:`NewEnumerator1`
      _))
  (`self.Possess` _returnvalue)
  (return _returnvalue))

(fn `UserConstructionScript`)