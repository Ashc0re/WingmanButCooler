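; Player controller for the main menu, which clears any online session and presents the menu on BeginPlay.
; BeginPlay calls DestroySession and, from its immediate output rather than its success callback, triggers two client events.
; One creates WBP_MainMenu, adds it to the viewport and switches input to UI only with the widget focused.
; The other sets the view target to the first BP_C_Main actor found in the level.
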(event `self.ReceiveBeginPlay`
  ;[1 1 1] Create main menu widget and set new view target
  (`DestroySessionCallbackProxy.DestroySession` self
    (:`then`
      (`self.Client_CreateMainMenuWidget`)
      (`self.Client_SetNewViewTarget`))))

(event `Client_SetNewViewTarget`
  ;[1 1 1] Set new view target
  (bind _outactors (`GameplayStatics.GetAllActorsOfClass` "/Game/Blueprints/Cameras/BP_C_Main.BP_C_Main_C"))
  (`self.SetViewTargetWithBlend` (`|GetArrayItem` _outactors)))

(event `Client_CreateMainMenuWidget`
  ;[1 1 1] Create main menu widget
  (bind _returnvalue (`|CreateWidget` "/Game/Widgets/MultiplayerWidgets/WBP_MainMenu.WBP_MainMenu_C"))
  (`UserWidget.AddToViewport` _returnvalue 0)
  (`WidgetBlueprintLibrary.SetInputMode_UIOnlyEx` (`GameplayStatics.GetPlayerController` 0) _returnvalue))

(fn `UserConstructionScript`)