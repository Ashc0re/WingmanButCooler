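; Bomb weapon for the Defusal game mode that handles timed planting on bomb sites.
; Trigger requires no planted bomb, an In Round or Post Round match state, and an owner overlapping a BombSite-tagged actor.
; It starts a looping progress timer and immediately pays one team's players currency.
; Reaching PlantTime sends the owner's plant message; Cancel resets progress, and replicated Timer updates drive the owner's InteractProgress.
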(fn `Cancel`
  (`KismetSystemLibrary.K2_ClearTimer` null "UpdateProgress")
  (set `self.Timer` 0.0))

(fn `OnRep_Timer`
  (bind _asbp_player_defusal (cast `/Game/Blueprints/Characters/BP_Player_Defusal` (`self.GetOwner`)))
  (set `/Game/Blueprints/Characters/BP_Player_Defusal.Interact Progress` (/ (`self.Timer`) (`self.PlantTime`)) _asbp_player_defusal))

(fn `Trigger`
  (params (`Camera Transform` :type "Transform Structure"))
  (locals (IsOnBombSite :type Boolean) (`Game State` :type "/Game/Blueprints/Gamestate/GS_Defusal Object Reference"))
  (bind _asgs_defusal (cast `/Game/Blueprints/Gamestate/GS_Defusal` (`GameplayStatics.GetGameState`)))
  (bind _output_get (set `local.Game State` _asgs_defusal))
  (if (not (`/Game/Blueprints/Gamestate/GS_Defusal.IsBombPlanted` _output_get))
    (switch `/Game/Blueprints/Controllers/Enum_MatchState` (`/Game/Blueprints/Gamestate/GS_Defusal.MatchState` (`local.Game State`))
      (:`NewEnumerator2`
        _)
      (:`NewEnumerator3`
        _))
    (bind _outactors (`GameplayStatics.GetAllActorsWithTag` "BombSite"))
    (for _array_element _outactors
      (if (`Actor.IsOverlappingActor` (`self.GetOwner`) _array_element)
        (set `local.IsOnBombSite` true)))
    (if (`local.IsOnBombSite`)
      (`KismetSystemLibrary.K2_SetTimer` null "UpdateProgress" 0.01 true true)
      (bind _outactors_2 (`GameplayStatics.GetAllActorsOfClass` "/Game/Blueprints/Characters/BP_Player_Defusal.BP_Player_Defusal_C"))
      (for _array_element_2 _outactors_2
        (if (`|EnumEquality` (`/Game/Blueprints/Characters/BP_Player_Defusal.Team` _array_element_2) "NewEnumerator0")
          (`/Game/Blueprints/Characters/BP_Player_Defusal.Server_AddCurrency` _array_element_2 300))))))

(fn `UpdateProgress`
  (bind _output_get (set `self.Timer` (+ (`self.Timer`) 0.01)))
  (if (>= _output_get (`self.PlantTime`))
    (`self.Cancel`)
    (message `/Game/Blueprints/Interfaces/BPI_Player.PlantBomb` (`self.GetOwner`))))