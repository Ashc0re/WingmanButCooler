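; Base weapon Blueprint owned by BP_Player that handles hitscan firing with ammo and per-body-part damage.
; TriggerWeapon passes a camera transform to FireWeapon, which checks CanFire and ammo, plays firing animations, and sphere-traces forward with debug drawing.
; Hits skip player capsules, register once per player, and use physical material surface types to pick head, torso or limb damage for ServerDealDamage.
; Same-team hits only print a message.
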(event `TriggerWeapon`
  (params (`Camera Transform` :type "Transform Structure"))
  (`self.Fire Weapon` `Camera Transform`))

(event `self.ReceiveBeginPlay`
  (bind _asbp_player (cast `/Game/Blueprints/Characters/BP_Player` (`self.GetOwner`)))
  (set `self.Owning Player` _asbp_player))

(fn `Fire Weapon`
  (params (`Camera Transform` :type "Transform Structure"))
  (locals (`Sphere Trace Objects` :type "Array of EObjectTypeQuery Enum") (`Out Hit Surface Type` :type "EPhysicalSurface Enum" :default "SurfaceType3"))
  (bind _location (.location `Camera Transform`))
  (if (`/Game/Blueprints/Characters/BP_Player.CanFire?` (`self.Owning Player`))
    (if (> (`self.CurrentAmmo`) 0)
      (`/Engine/EditorBlueprintResources/StandardMacros.DecrementInt` (`self.CurrentAmmo`)
        (:`  `
          (`|ExecutionSequence`
            (:`then_0`
              (`self.PlayAnimation` (`/Game/Blueprints/Characters/BP_Player.ThirdPersonGun` (`self.Owning Player`)) (`self.FireringAnimation`) false))
            (:`then_1`
              (`self.PlayAnimation` (`self.FireringAnimation`)))
            (:`then_2`
              (bind _outhits (`KismetSystemLibrary.SphereTraceMultiForObjects` :`Start` _location :`End` (+ _location (* (`KismetMathLibrary.GetForwardVector` (.rotation `Camera Transform`)) (`self.Range`))) :`Radius` 2.0 :`ObjectTypes` (`local.Sphere Trace Objects`) :`bTraceComplex` true :`DrawDebugType` "ForDuration"))
              (`KismetArrayLibrary.Array_Clear` (`self.Hit Actors`))
              (for _array_element _outhits
                (bind (_bblockinghit _binitialoverlap _time _distance _location_2 _impactpoint _normal _impactnormal _physmat _hitactor _hitcomponent) (`GameplayStatics.BreakHitResult` _array_element))
                (set `local.Out Hit Surface Type` (`PhysicalMaterial.SurfaceType` _physmat))
                (if (`GameplayStatics.ObjectIsA` _hitactor "/Game/Blueprints/Characters/BP_Player.BP_Player_C")
                  (if (`GameplayStatics.ObjectIsA` _hitcomponent "/Script/Engine.CapsuleComponent")
                    _
                    (elif (not (`KismetArrayLibrary.Array_Contains` (`self.Hit Actors`) _hitactor))
                      (`KismetArrayLibrary.Array_Add` (`self.Hit Actors`) _hitactor)
                      (bind _asbp_player (cast `/Game/Blueprints/Characters/BP_Player` _hitactor))
                      (if (`|EnumInequality` (`/Game/Blueprints/Characters/BP_Player.Team` _asbp_player) (`/Game/Blueprints/Characters/BP_Player.Team` (`self.Owning Player`)))
                        (switch `EPhysicalSurface` (`local.Out Hit Surface Type`)
                          (:`SurfaceType1`
                            (`/Game/Blueprints/Characters/BP_Player.Server_DealDamage` _asbp_player (`self.DamageHead`)))
                          (:`SurfaceType2`
                            (`/Game/Blueprints/Characters/BP_Player.Server_DealDamage` _asbp_player (`self.DamageTorso`)))
                          (:`SurfaceType3`
                            (`/Game/Blueprints/Characters/BP_Player.Server_DealDamage` _asbp_player (`self.DamageLimb`))))
                        (else
                          (`KismetSystemLibrary.PrintString` "Friendly Hit!"))))))))))))))