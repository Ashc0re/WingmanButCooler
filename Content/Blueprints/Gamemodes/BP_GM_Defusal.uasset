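; Game mode for a Terror versus Anti-Terror bomb defusal match, running warmup, preparing, round, post-round and game-over states.
; A reversed timeline serves as the countdown that advances states; expired rounds go to Anti-Terror, eliminations end them early.
; Round wins grant team currency and score toward game over, while preparation cleans up and respawns everyone.
; Spawning reserves team-tagged PlayerStarts, then equips pistols, plus bombs for Terrorists.
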(event `self.ReceiveBeginPlay`
  (bind _asgs_defusal (cast `/Game/Blueprints/Gamestate/GS_Defusal` (`GameplayStatics.GetGameState`)))
  (set `self.Defusal Game State` _asgs_defusal)
  (`self.TimerSet` 30.0)
  (`self.TimerResume`))

(event `Server_AddPlayerToTeam`
  (params (IsTerrorPlayer :type Boolean))
  (if IsTerrorPlayer
    (`/Engine/EditorBlueprintResources/StandardMacros.IncrementInt` (`/Game/Blueprints/Gamestate/GS_Defusal.TotalTerrorPlayers` (`self.Defusal Game State`)))
    (else
      (`/Engine/EditorBlueprintResources/StandardMacros.IncrementInt` (`/Game/Blueprints/Gamestate/GS_Defusal.TotalAntiTerrorPlayers` (`self.Defusal Game State`))))))

(event `Server_ReturnToLobby`
  ;[1 1 1] Return to lobby on server
  (for _array_element (`self.AllGameplayPlayers`)
    (`/Game/Blueprints/Controllers/BP_PC_Defusal.Client_CreateLoadingScreen` _array_element))
  (`KismetSystemLibrary.ExecuteConsoleCommand` (`KismetStringLibrary.Concat_StrStr` "servertravel /Levels/Menus/" "Lobby") null))

(event `self.HandleStartingNewPlayer`
  (params (NewPlayer :type "PlayerController Object Reference"))
  ;[1 1 1] Add new player to "AllGameplayPlayers"
  (bind _asbp_pc_defusal (cast `/Game/Blueprints/Controllers/BP_PC_Defusal` NewPlayer))
  (`KismetArrayLibrary.Array_Add` (`self.AllGameplayPlayers`) _asbp_pc_defusal))

(event `TimerStop`
  (bind (_direction _warmup_timer) (`Timeline|Timeline_MatchTimer` :`NewTime` (stale `TimerSet` NewTime) :!via `Stop` :!label _label)
    (:`Update`
      (set `self.Timer` (`KismetMathLibrary.FTrunc` _warmup_timer))
      (switch `/Game/Blueprints/Controllers/Enum_MatchState` (`self.MatchState`)
        (:`NewEnumerator0`
          (`self.GameLogicWarmup`))))
    (:`Finished`
      (switch `/Game/Blueprints/Controllers/Enum_MatchState` (`self.MatchState`)
        (:`NewEnumerator0`
          (`self.StartMatch`))
        (:`NewEnumerator1`
          (`self.StartRound`))
        (:`NewEnumerator2`
          (`self.StartPostRund` "NewEnumerator1"))
        (:`NewEnumerator3`
          (`self.StartPreparing`))))))

(event `/Game/Blueprints/Interfaces/BPI_MatchLogic.SpawnPlayerOfTeam`
  (params (Team :type "/Game/Blueprints/Characters/Enum_Team Enum" :default "NewEnumerator0") (`Player Controller` :type "PlayerController Object Reference"))
  ;[0.15 0.15 0.15] Spawning of Players
  ;;[0.15 0.15 0.15] Spawn Player of a given Team - AC
  (`self.SpawnCharacter` Team `Player Controller`))

(event `TimerResume`
  (goto _label :!via `Reverse`))

(event `TimerStart`
  (goto _label :!via `ReverseFromEnd`))

(event `TimerSet`
  (params (NewTime :type "Float (single-precision)"))
  (goto _label :!via `SetNewTime`))

(event `GameLogicWarmup`
  (`|ExecutionSequence`
    (:`then_0`
      (if (and (>= (`/Game/Blueprints/Gamestate/GS_Defusal.TotalTerrorPlayers` (`self.Defusal Game State`)) 1) (>= (`/Game/Blueprints/Gamestate/GS_Defusal.TotalAntiTerrorPlayers` (`self.Defusal Game State`)) 1))
        (`/Engine/EditorBlueprintResources/StandardMacros.DoOnce` false
          (:`Completed`
            (`self.TimerStop`)
            (`self.TimerSet` 20.0)
            (`self.TimerResume`)))))
    (:`then_1`
      (if (and (== (`/Game/Blueprints/Gamestate/GS_Defusal.TotalTerrorPlayers` (`self.Defusal Game State`)) 2) (== (`/Game/Blueprints/Gamestate/GS_Defusal.TotalAntiTerrorPlayers` (`self.Defusal Game State`)) 2))
        (`/Engine/EditorBlueprintResources/StandardMacros.DoOnce` false
          (:`Completed`
            (`self.TimerStop`)
            (`self.TimerSet` 5.0)
            (`self.TimerResume`)))))))

(event `/Game/Blueprints/Interfaces/BPI_MatchLogic.PlayerDeath`
  (params (`Player State` :type "PlayerState Object Reference") (Team :type "/Game/Blueprints/Characters/Enum_Team Enum" :default "NewEnumerator0") (Controller :type "Controller Object Reference"))
  (bind _defusal_game_state (`self.Defusal Game State`))
  ;[0.15 0.15 0.15] Spawning of Players
  ;;[0.15 0.15 0.15] Handles Dead Players and Respawns - AC
  (`BlueprintMapLibrary.Map_Add` (`self.AllDeadPlayers`) `Player State` Team)
  (switch `/Game/Blueprints/Characters/Enum_Team` Team
    (:`NewEnumerator0`
      (`/Engine/EditorBlueprintResources/StandardMacros.DecrementInt` (`/Game/Blueprints/Gamestate/GS_Defusal.AliveTerrorPlayers` _defusal_game_state)
        (:`  `
          _)))
    (:`NewEnumerator1`
      (`/Engine/EditorBlueprintResources/StandardMacros.DecrementInt` (`/Game/Blueprints/Gamestate/GS_Defusal.AliveAntiTerrorPlayers` _defusal_game_state)
        (:`  `
          _))))
  (switch `/Game/Blueprints/Controllers/Enum_MatchState` (`self.MatchState`)
    (:`NewEnumerator0`
      (bind _asbp_pc_defusal (cast `/Game/Blueprints/Controllers/BP_PC_Defusal` Controller))
      (`self.Player Respawn` _asbp_pc_defusal)
      (`/Engine/EditorBlueprintResources/StandardMacros.FlipFlop`
        (:`A`
          (if true
            (`self.ResetSpawnPoints`)))))
    (:`NewEnumerator2`
      (`self.CheckForEleminationWin`))))

(event `/Game/Blueprints/Interfaces/BPI_MatchLogic.Player Respawn`
  (params (`Player Controller` :type "PlayerController Object Reference"))
  (bind _playerstate (`Controller.PlayerState` `Player Controller`))
  (bind (_value _returnvalue) (`BlueprintMapLibrary.Map_Find` (`self.AllDeadPlayers`) _playerstate))
  ;[0.15 0.15 0.15] Spawning of Players
  ;;[0.15 0.15 0.15] Handles Dead Players and Respawns - AC
  (if _returnvalue
    (`self.SpawnPlayerOfTeam` _value `Player Controller`)
    (`BlueprintMapLibrary.Map_Remove` (`self.AllDeadPlayers`) _playerstate)
    (else
      (`KismetSystemLibrary.PrintString` "This player isn't dead!"))))

(event `/Game/Blueprints/Interfaces/BPI_MatchLogic.StartMatch`
  (if (`|EnumEquality` (`self.MatchState`) "NewEnumerator0")
    (`self.TimerStop`)
    (`self.StartPreparing`)
    (else
      (`KismetSystemLibrary.PrintString` "Match already in progress!"))))

(event `StartPreparing`
  (`self.TimerStop`)
  (set `self.MatchState` "NewEnumerator1")
  (`self.ToggleMovementModeForAllPlayers` false)
  (`self.CleanUp`)
  (`self.TimerSet` 10.0)
  (`self.TimerResume`))

(event `StartRound`
  (set `self.MatchState` "NewEnumerator2")
  (`self.ToggleMovementModeForAllPlayers` true)
  (`self.TimerSet` 300.0)
  (`self.TimerResume`))

(event `StartPostRund`
  (params (Winner :type "/Game/Blueprints/Characters/Enum_Team Enum" :default "NewEnumerator0"))
  (`self.TimerStop`)
  (bind _ismatchwon_ (`self.RoundWon` Winner))
  (if _ismatchwon_
    (`self.StartGameOver` Winner)
    (else
      (set `self.MatchState` "NewEnumerator3")
      (`self.TimerSet` 5.0)
      (`self.TimerResume`))))

(event `StartGameOver`
  (params (Winner :type "/Game/Blueprints/Characters/Enum_Team Enum" :default "NewEnumerator0"))
  (set `self.MatchState` "NewEnumerator4")
  (`self.ToggleMovementModeForAllPlayers` false)
  (`KismetSystemLibrary.Delay` 5.0)
  (for _array_element (`self.AllGameplayPlayers`)
    (`DestroySessionCallbackProxy.DestroySession` _array_element
      (:`then`
        (`GameplayStatics.OpenLevelBySoftObjectPtr` "/Game/Levels/Menus/MainMenu.MainMenu")))))

(event `CleanUp`
  (`|ExecutionSequence`
    (:`then_0`
      (`self.KillRemainingPlayers`))
    (:`then_1`
      (`self.RemoveWeaponPickups`))
    (:`then_2`
      (`self.RemovePlantedBombs`))
    (:`then_3`
      (`self.ResetSpawnPoints`))
    (:`then_4`
      (`self.RespawnAllPlayers`))))

(event `Multicast_KillPlayer`
  (params (Player :type "/Game/Blueprints/Characters/BP_Player_Defusal Object Reference"))
  (`/Game/Blueprints/Characters/BP_Player_Defusal.Server_PlayerDeath` Player))

(event `Multicast_DestroyActor`
  (params (ActorToDestroy :type "Actor Object Reference"))
  (`self.K2_DestroyActor` ActorToDestroy))

(fn `CheckForEleminationWin`
  (if (<= (`/Game/Blueprints/Gamestate/GS_Defusal.AliveTerrorPlayers` (`self.Defusal Game State`)) 0)
    (`self.StartPostRund` "NewEnumerator1")
    (elif (<= (`/Game/Blueprints/Gamestate/GS_Defusal.AliveAntiTerrorPlayers` (`self.Defusal Game State`)) 0)
      (`self.StartPostRund` "NewEnumerator0"))))

(fn `GetRandomSpawnOfTeam`
  (params (Team :type "/Game/Blueprints/Characters/Enum_Team Enum" :default "NewEnumerator0") (`Reset Spawn Points` :type Boolean))
  (returns (ReturnValue :type "Transform Structure (by ref)"))
  (bind _outactors (`GameplayStatics.GetAllActorsOfClassWithTag` "/Script/Engine.PlayerStart" (`KismetStringLibrary.Conv_StringToName` (`KismetStringLibrary.Conv_ByteToString` Team))))
  (for _array_element _outactors
    (if `Reset Spawn Points`
      (set `PlayerStart.PlayerStartTag` "Reserved" _array_element))
    (if (!= (`PlayerStart.PlayerStartTag` _array_element) "Reserved")
      (set `PlayerStart.PlayerStartTag` "Reserved" _array_element)
      (break)))
  (return (`self.GetTransform` _array_element)))

(fn `GrantWinnerCurrency`
  (params (Winner :type "/Game/Blueprints/Characters/Enum_Team Enum" :default "NewEnumerator0") (CurrencyToAdd :type Integer))
  (for _array_element (`self.AllGameplayPlayers`)
    (bind _team (`/Game/Blueprints/Controllers/BP_PC_Defusal.GetTeam` _array_element))
    (if (`|EnumEquality` _team Winner)
      (`/Game/Blueprints/Controllers/BP_PC_Defusal.AddCurrency` _array_element CurrencyToAdd))))

(fn `OnRep_MatchState`
  (set `/Game/Blueprints/Gamestate/GS_Defusal.MatchState` (`self.MatchState`) (`self.Defusal Game State`)))

(fn `OnRep_Timer`
  (set `/Game/Blueprints/Gamestate/GS_Defusal.Timer` (`self.Timer`) (`self.Defusal Game State`)))

(fn `ResetSpawnPoints`
  (bind _outactors (`GameplayStatics.GetAllActorsOfClass` "/Script/Engine.PlayerStart"))
  (for _array_element _outactors
    (set `PlayerStart.PlayerStartTag` "None" _array_element)))

(fn `RoundWon`
  (params (Winner :type "/Game/Blueprints/Characters/Enum_Team Enum" :default "NewEnumerator0"))
  (returns (`IsMatchWon?` :type Boolean))
  (bind _defusal_game_state (`self.Defusal Game State`))
  (`self.GrantWinnerCurrency` Winner 500)
  (switch `/Game/Blueprints/Characters/Enum_Team` Winner
    (:`NewEnumerator0`
      (bind _result (`/Engine/EditorBlueprintResources/StandardMacros.IncrementInt` (`/Game/Blueprints/Gamestate/GS_Defusal.ScoreTerror` _defusal_game_state))
        (:`  `
          (if (>= _result (`self.RoundsToWin`))
            _
            (else
              (return false))))))
    (:`NewEnumerator1`
      (bind _result_2 (`/Engine/EditorBlueprintResources/StandardMacros.IncrementInt` (`/Game/Blueprints/Gamestate/GS_Defusal.ScoreAntiTerror` _defusal_game_state))
        (:`  `
          (if (>= _result_2 (`self.RoundsToWin`))
            _
            (else
              (return false)))))))
  (return true))

(fn `SpawnCharacter`
  (params (Team :type "/Game/Blueprints/Characters/Enum_Team Enum" :default "NewEnumerator0") (`Player Controller` :type "Controller Object Reference"))
  (locals (_PlayerController :type "Controller Object Reference") (_Team :type "/Game/Blueprints/Characters/Enum_Team Enum" :default "NewEnumerator0") (_Player :type "/Game/Blueprints/Characters/BP_Player_Defusal Object Reference") (_Spawnpoint :type "PlayerStart Object Reference"))
  ;[0.15 0.15 0.15] Find free player start and spawn player
  (set `local._PlayerController` `Player Controller`)
  (bind _output_get (set `local._Team` Team))
  (bind _outactors (`GameplayStatics.GetAllActorsOfClassWithTag` "/Script/Engine.PlayerStart" (`KismetStringLibrary.Conv_StringToName` (`|GetEnumeratorNameAsString` _output_get))))
  (for _array_element _outactors
    (bind _output_get_2 (set `local._Spawnpoint` _array_element))
    (if (!= (`PlayerStart.PlayerStartTag` _output_get_2) "Reserved")
      (set `PlayerStart.PlayerStartTag` "Reserved" (`local._Spawnpoint`))
      (break)))
  (bind __spawnpoint (`local._Spawnpoint`)
    (:`then`
      (bind _returnvalue (`|SpawnActorFromClass` "/Game/Blueprints/Characters/BP_Player_Defusal.BP_Player_Defusal_C" (`self.GetTransform` __spawnpoint) "AdjustIfPossibleButAlwaysSpawn" "MultiplyWithRoot" null null))
      (bind _output_get_3 (set `local._Player` _returnvalue))
      (bind _output_get_4 (set `/Game/Blueprints/Characters/BP_Player_Defusal.Team` (`local._Team`) _output_get_3))
      (switch `/Game/Blueprints/Characters/Enum_Team` _output_get_4
        (:`NewEnumerator0`
          (`self.Server_AddPlayerToTeam` true)
          (set `/Game/Blueprints/Characters/BP_Player_Defusal.Skin` "/Game/3D/ThirdPersonCharacter/Materials/MI_UE4Man_Body_Terror.MI_UE4Man_Body_Terror" (`local._Player`))
          (`/Game/Blueprints/Characters/BP_Player_Defusal.CreateWeapon` (`local._Player`) "/Game/Blueprints/Weapons/BP_Bomb.BP_Bomb_C" (0.0 0.0 0.0) 0 0))
        (:`NewEnumerator1`
          (`self.Server_AddPlayerToTeam` false)
          (set `/Game/Blueprints/Characters/BP_Player_Defusal.Skin` "/Game/3D/ThirdPersonCharacter/Materials/MI_UE4Man_Body_AntiTerror.MI_UE4Man_Body_AntiTerror" (`local._Player`))))
      (`/Game/Blueprints/Characters/BP_Player_Defusal.CreateWeapon` (`local._Player`) "/Game/Blueprints/Weapons/BP_Pistol.BP_Pistol_C" (0.0 0.0 0.0) 12 36)
      (`Controller.Possess` (`local._PlayerController`) (`local._Player`)))
    (:`else`
      (`KismetSystemLibrary.PrintString` "Error: No Spawnpoint Found" true true (struct :`R` 1.0 :`G` 0.1 :`B` 0.1 :`A` 1.0) 5.0))))

(fn `ToggleMovementModeForAllPlayers`
  (params (CanMove :type Boolean))
  (for _array_element (`self.AllGameplayPlayers`)
    (`/Game/Blueprints/Controllers/BP_PC_Defusal.SetMovementMode` _array_element CanMove)))

(fn `UserConstructionScript`)