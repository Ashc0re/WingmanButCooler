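; Lobby game mode that tracks joined player controllers and handles map info, the player list, kicking and match start.
; On join it has the client create its HUD and character, then pushes map info, seeded from the "Default" D_Maps row if empty, and rebuilds every client's player list.
; Logout removes the controller and refreshes the list.
; Starting the game shows loading screens, then runs servertravel to the selected map under the Defusal levels folder.
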(event `Server_KickPlayerFromTheLobby`
  (params (PlayerLobbyIndex :type Integer))
  ;[1 1 1] Kick player from the lobby
  (`/Game/Blueprints/Controllers/BP_PC_Lobby.Client_KickPlayerFromTheLobby` (`|GetArrayItem` (`self.AllLobbyPlayers`) PlayerLobbyIndex)))

(event `self.HandleStartingNewPlayer`
  (params (NewPlayer :type "PlayerController Object Reference"))
  ;[1 1 1] Create lobby widget and update lobby information
  (bind _asbp_pc_lobby (cast `/Game/Blueprints/Controllers/BP_PC_Lobby` NewPlayer))
  (`KismetArrayLibrary.Array_Add` (`self.AllLobbyPlayers`) _asbp_pc_lobby)
  (`/Game/Blueprints/Controllers/BP_PC_Lobby.Client_CreateHUDAndSpawnCharacter` _asbp_pc_lobby)
  (`self.UpdateMapInfoForAllClients` (`self.Maps`))
  (`self.Server_UpdateLobbyPlayerlist`))

(event `Server_StartGame`
  ;[1 1 1] Start match and server travel into level
  (`self.ServerTravelIntoLevel`))

(event `Server_UpdateServerInfoOnClients`
  (params (S_Maps :type "/Game/Blueprints/Structures/S_Maps Structure"))
  ;[1 1 1] Update map information for all players
  (bind _output_get (set `self.Maps` S_Maps))
  (for _array_element (`self.AllLobbyPlayers`)
    (`/Game/Blueprints/Controllers/BP_PC_Lobby.Client_UpdateMapInfoOnHUD` _array_element _output_get)))

(event `Server_UpdateLobbyPlayerlist`
  ;[1 1 1] Update playerlist information on server
  (`self.UpdatePlayerlistInformation`))

(event `self.K2_OnLogout`
  (params (ExitingController :type "Controller Object Reference"))
  ;[1 1 1] Logout player when kicked or disconnect
  (`self.LogoutUserWhenDisconnecting` ExitingController))

(fn `LogoutUserWhenDisconnecting`
  (params (InputPin :type "Controller Object Reference"))
  ;[1 1 1] Logout User, remove player from "AllLobbyPlayers", update playerlist
  (for (_array_element _array_index) (`self.AllLobbyPlayers`)
    (if (== _array_element InputPin)
      (break)))
  (`KismetArrayLibrary.Array_Remove` (`self.AllLobbyPlayers`) _array_index)
  (`self.Server_UpdateLobbyPlayerlist`))

(fn `ServerTravelIntoLevel`
  ;[1 1 1] Show loading screens for the players and server travel into llevel
  (for _array_element (`self.AllLobbyPlayers`)
    (`/Game/Blueprints/Controllers/BP_PC_Lobby.Client_CreateLoadingScreen` _array_element))
  (`KismetSystemLibrary.ExecuteConsoleCommand` (`KismetStringLibrary.Concat_StrStr` "servertravel /Game/Levels/Defusal/" (`.MapServerTravel_10_ABE1869A49AC3B78614CF6BBD72FF46E` (break `/Game/Blueprints/Structures/S_Maps` (`self.Maps`)))) null))

(fn `UpdateMapInfoForAllClients`
  (params (CurrentMap :type "/Game/Blueprints/Structures/S_Maps Structure"))
  ;[1 1 1] Get default map from datatable and update it for all clients
  (if (`KismetStringLibrary.EqualEqual_StrStr` (`.MapName_12_78E99B0D4B5170E0248315940147EEE6` (break `/Game/Blueprints/Structures/S_Maps` (`self.Maps`))))
    (bind _returnvalue (`|GetDataTableRow` "/Game/Blueprints/Datatables/D_Maps.D_Maps" "Default")
      (:`then`
        (bind _output_get (set `self.Maps` _returnvalue))
        (`self.Server_UpdateServerInfoOnClients` _output_get)))
    (else
      (bind _output_get_2 (set `self.Maps` CurrentMap))
      (`self.Server_UpdateServerInfoOnClients` _output_get_2))))

(fn `UpdatePlayerlistInformation`
  (bind _alllobbyplayers (`self.AllLobbyPlayers`))
  ;[1 1 1] Clear all players from the list and update list with new players
  (for _array_element _alllobbyplayers
    (`/Game/Blueprints/Controllers/BP_PC_Lobby.Client_ClearAllPlayersFromTheList` _array_element)
    (for (_array_element_2 _array_index) _alllobbyplayers
      (`/Game/Blueprints/Controllers/BP_PC_Lobby.Client_AddNewPlayerToList` _array_element (`PlayerState.GetPlayerName` (`Controller.PlayerState` _array_element_2)) _array_index))))

(fn `UserConstructionScript`)